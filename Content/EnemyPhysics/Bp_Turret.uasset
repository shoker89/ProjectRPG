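; Turret Blueprint meant to fire physics-driven BP_Projectile actors at a fixed rate.
; The shot spawns a projectile at SpawnProjectilePosition and pushes its Sphere along the Arrow's forward vector with a mass-independent force.
; A CanShoot flag and a Delay throttle shots to about one per second.
; The firing logic hangs off a Timeline update that nothing starts, so it never runs as written.
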(fn ConstructionScript)