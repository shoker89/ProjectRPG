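; HandlingDamage is an animation notify state that performs hit detection and damage during its window in an animation.
; Each tick it sphere-traces on the Visibility channel between two mesh sockets, printing hit component names.
; The first named hit component is passed to its actor through HitLocationMessage, ending the loop.
; ApplyDamage then runs after the loop on the current element's actor every tick, with no guard against repeat hits.
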(fn ReceivedNotifyTick
  (params (MeshComp :type Skeletal%20Mesh%20Component%20Object%20Reference) (Animation :type Anim%20Sequence%20Base%20Object%20Reference) (FrameDeltaTime :type Float%20%28single-precision%29))
  (bind _outhits (Collision|MultiSphereTraceByChannel MeshComp (Transformation|GetSocketLocation MeshComp (Variables|Default|GetSocketNameStart)) (Transformation|GetSocketLocation MeshComp (Variables|Default|GetSocketNameEnd)) 1e+01 "TraceTypeQuery1" false 0 "None"))
  (bind _array_element (Utilities|Array|ForEachLoopwithBreak _outhits :!label _label)
    (:LoopBody
      (Development|PrintString 0 (Utilities|String|Append "Sphere hit: " (Utilities|GetDisplayName (.hitcomponent _array_element))))
      (if (not (Utilities|Array|IsEmpty (Utilities|GetDisplayName (.hitcomponent _array_element))))
        (Class|CombatInterface|HitLocation(Message) (.hitactor _array_element) (.hitcomponent _array_element))
        (goto _label Break)))
    (:Completed
      (Game|Damage|ApplyDamage (.hitactor _array_element) 1e+01 0 0)
      (return false))))